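; Lobby character Blueprint that puts the authentication UI on screen.
; On BeginPlay with authority, it calls AddAuthWidgetOnClient, which waits briefly, then constructs BP_AuthenticationUI for the first player controller and adds it to the viewport.
; Nodes to show the mouse cursor, store the widget, link it back to the character and set its owning player are disconnected and never run.
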(event Custom|AddAuthWidgetOnClient
  (Utilities|FlowControl|Delay 1.0)
  (bind _returnvalue (Game|ConstructObjectfromClass "/Game/Lobby/BP_AuthenticationUI.BP_AuthenticationUI_C" (Game|GetPlayerController 0)))
  (UserInterface|Viewport|AddtoViewport _returnvalue 0))

(event EventBeginPlay
  (Networking|SwitchHasAuthority
    (:Authority
      (CallFunction|AddAuthWidgetonClient))))

(fn ConstructionScript)