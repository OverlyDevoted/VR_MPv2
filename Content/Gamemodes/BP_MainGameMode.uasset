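; Main game mode that gates players behind a code-based authentication step before giving them a playable character.
; After a short delay, PostLogin records the new player on the server, then spawns and possesses an indexed BP_AuthenticationCharacter for them.
; Authenticate compares the submitted code to admin and user codes, spawning and possessing a different character for each role.
; An unrecognized code only prints debug messages, and the submitted name goes unused.
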(event Custom|SpawnAuthenticationOnServer
  (CallFunction|SpawnAuthenticationonClient))

(event Custom|SpawnAuthenticationOnClient
  (Development|PrintString (Utilities|String|Append (Class|AdvancedSessionsLibrary|GetPlayerName (stale EventPostLogin NewPlayer)) " " (Utilities|String|ToString(Integer) (stale EventPostLogin _returnvalue))))
  (bind _returnvalue (Game|SpawnActorfromClass "/Game/Lobby/BP_AuthenticationCharacter.BP_AuthenticationCharacter_C" (Math|Transform|MakeTransform "0,1000.000000, 0" "0, 0, 0" "1,1,1") "AlwaysSpawn" (stale EventPostLogin NewPlayer) (stale EventPostLogin _returnvalue) 0))
  (Pawn|Possess (stale EventPostLogin NewPlayer) _returnvalue))

(event Custom|Authenticate
  (params (NewName :type String) (Code :type String) (PlayerController :type Player%20Controller%20Object%20Reference))
  (if (Utilities|Enum|Equal(Enum) Code (Variables|Default|GetAdminCode))
    (bind _returnvalue (Game|SpawnActorfromClass "/Game/ThirdPersonBP/Blueprints/ThirdPersonCharacter.ThirdPersonCharacter_C" (Math|Transform|MakeTransform "0, 0, 0" "0, 0, 0" "1,1,1") "AlwaysSpawn" PlayerController 0))
    (CallFunction|ClientPossess PlayerController _returnvalue)
    (else
      (Development|PrintString "Not admin")
      (if (Utilities|Enum|Equal(Enum) Code (Variables|Default|GetUserCode))
        (bind _returnvalue_2 (Game|SpawnActorfromClass "/Game/ThirdPersonBP/Blueprints/BP_TPCharacter.BP_TPCharacter_C" (Math|Transform|MakeTransform "0, 0, 0" "0, 0, 0" "1,1,1") "AlwaysSpawn" PlayerController 0))
        (CallFunction|ClientPossess PlayerController _returnvalue_2)
        (else
          (Development|PrintString "Not user"))))))

(event Custom|ClientPossess
  (params (Client :type Player%20Controller%20Object%20Reference) (Pawn :type Pawn%20Object%20Reference))
  (Development|PrintString (Utilities|String|Append "on game mode" " " (Class|AdvancedSessionsLibrary|GetPlayerName Client)))
  (Pawn|Possess Client Pawn))

(event EventPostLogin
  (params (NewPlayer :type Player%20Controller%20Object%20Reference))
  (Networking|SwitchHasAuthority
    (:Authority
      (Utilities|FlowControl|Delay 1.0)
      (bind _returnvalue (Utilities|Array|Add (Variables|Default|GetPlayers) NewPlayer))
      (CallFunction|SpawnAuthenticationonServer))))

(fn ConstructionScript)